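; Interactable two-way door that RememberCharacter opens with the Interact input from either of two trigger boxes and that closes after they leave.
; Each box enables input and opens its gate, and interacting plays a timeline rotating the door's yaw, negated for the second side.
; Opening disables the opposite box's flag until closing finishes.
; Leaving the active box reverses a close timeline after a short delay, with separate timelines for mid-animation exits.
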(event OnComponentBeginOverlap(DoorHitbox1)
  (params (OverlappedComponent :type Primitive%20Component%20Object%20Reference) (OtherActor :type Actor%20Object%20Reference) (OtherComp :type Primitive%20Component%20Object%20Reference) (OtherBodyIndex :type Integer) (bFromSweep :type Boolean) (SweepResult :type Hit%20Result%20Structure%20%28by%20ref%29))
  ;[1 1 1] Checking overlaps with RememberCharacter actors only
  (Utilities|Casting|CastToRememberCharacter OtherActor)
  (Variables|Default|SetGateLock1 true)
  (if (Variables|Default|GetHitbox1Enabled)
    ;[1 1 1] If player interacts with the door and the door is not moving or closed
    (Input|EnableInput (Game|GetPlayerController 0))
    (Utilities|FlowControl|Gate true) ; enters at Open
  ))

(event OnComponentEndOverlap(DoorHitbox1)
  (params (OverlappedComponent :type Primitive%20Component%20Object%20Reference) (OtherActor :type Actor%20Object%20Reference) (OtherComp :type Primitive%20Component%20Object%20Reference) (OtherBodyIndex :type Integer))
  ;[1 1 1] Checking overlaps with RememberCharacter actors only
  (Utilities|Casting|CastToRememberCharacter OtherActor)
  (Variables|Default|SetGateLock1 false)
  (if (Variables|Default|GetHitbox1Enabled)
    ;[1 1 1] If player leaves the trigger box after animation is completed
    (Input|DisableInput (Game|GetPlayerController 0))
    (if (Variables|Default|GetIsMoving)
      ;[1 1 1] If player leaves trigger box before animation is completed
      (Utilities|FlowControl|Delay 0.6)
      (if (Variables|Default|GetIsOpen)
        (bind _doorrotation (Timeline|DoorCloseDelayed ReverseFromEnd)
          (:Update
            (Variables|Default|SetIsMoving true)
            (Transformation|SetRelativeRotation (Variables|Default|GetDoor) (Math|Rotator|MakeRotator 0.0 0.0 (+ _doorrotation (.yaw (Variables|Default|GetInitial%20Rotation)))) false false))
          (:Finished
            (Variables|Default|SetIsMoving false)
            (Variables|Default|SetIsOpen false)
            (Variables|Default|SetHitbox2Enabled true))))
      (elif (Variables|Default|GetIsOpen)
        (Utilities|FlowControl|Delay 0.6)
        (bind _doorrotation_2 (Timeline|DoorClose ReverseFromEnd)
          (:Update
            (Variables|Default|SetIsMoving true)
            (Transformation|SetRelativeRotation (Variables|Default|GetDoor) (Math|Rotator|MakeRotator 0.0 0.0 (+ _doorrotation_2 (.yaw (Variables|Default|GetInitial%20Rotation)))) false false))
          (:Finished
            (Variables|Default|SetIsMoving false)
            (Variables|Default|SetIsOpen false)
            (Variables|Default|SetHitbox2Enabled true)))))))

(event OnComponentBeginOverlap(DoorHitbox2)
  (params (OverlappedComponent :type Primitive%20Component%20Object%20Reference) (OtherActor :type Actor%20Object%20Reference) (OtherComp :type Primitive%20Component%20Object%20Reference) (OtherBodyIndex :type Integer) (bFromSweep :type Boolean) (SweepResult :type Hit%20Result%20Structure%20%28by%20ref%29))
  ;[1 1 1] Checking overlaps with RememberCharacter actors only
  (Utilities|Casting|CastToRememberCharacter OtherActor)
  (Variables|Default|SetGateLock2 true)
  (if (Variables|Default|GetHitbox2Enabled)
    ;[1 1 1] If player interacts with the door and the door is not moving or closed
    (Input|EnableInput (Game|GetPlayerController 0))
    (Utilities|FlowControl|Gate true) ; enters at Open
  ))

(event OnComponentEndOverlap(DoorHitbox2)
  (params (OverlappedComponent :type Primitive%20Component%20Object%20Reference) (OtherActor :type Actor%20Object%20Reference) (OtherComp :type Primitive%20Component%20Object%20Reference) (OtherBodyIndex :type Integer))
  ;[1 1 1] Checking overlaps with RememberCharacter actors only
  (Utilities|Casting|CastToRememberCharacter OtherActor)
  (Variables|Default|SetGateLock2 false)
  (if (Variables|Default|GetHitbox2Enabled)
    ;[1 1 1] If player leaves the trigger box after animation is completed
    (Input|DisableInput (Game|GetPlayerController 0))
    (if (Variables|Default|GetIsMoving)
      ;[1 1 1] If player leaves trigger box before animation is completed
      (Utilities|FlowControl|Delay 0.6)
      (if (Variables|Default|GetIsOpen)
        (bind _doorrotation (Timeline|DoorClosedDelayed2 ReverseFromEnd)
          (:Update
            (Variables|Default|SetIsMoving true)
            (Transformation|SetRelativeRotation (Variables|Default|GetDoor) (Class|KismetMathLibrary|NegateRotator (Math|Rotator|MakeRotator 0.0 0.0 (+ _doorrotation (.yaw (Variables|Default|GetInitial%20Rotation))))) false false))
          (:Finished
            (Variables|Default|SetIsMoving false)
            (Variables|Default|SetIsOpen false)
            (Variables|Default|SetHitbox1Enabled true))))
      (elif (Variables|Default|GetIsOpen)
        (Utilities|FlowControl|Delay 0.6)
        (bind _doorrotation_2 (Timeline|DoorClose2 ReverseFromEnd)
          (:Update
            (Variables|Default|SetIsMoving true)
            (Transformation|SetRelativeRotation (Variables|Default|GetDoor) (Class|KismetMathLibrary|NegateRotator (Math|Rotator|MakeRotator 0.0 0.0 (+ _doorrotation_2 (.yaw (Variables|Default|GetInitial%20Rotation))))) false false))
          (:Finished
            (Variables|Default|SetIsMoving false)
            (Variables|Default|SetIsOpen false)
            (Variables|Default|SetHitbox1Enabled true)))))))

(event EventBeginPlay)

(event Collision|EventActorBeginOverlap
  (params (OtherActor :type Actor%20Object%20Reference)))

(event Input|ActionEvents|InputActionInteract
  (params (Key :type Key%20Structure))
  ;[1 1 1] Check if gate can be opened
  (:Pressed
    (if (Variables|Default|GetGateLock2)
      ;[1 1 1] If player interacts with the door and the door is not moving or closed
      (Utilities|FlowControl|Gate true
        (:Exit
          (if (not (Variables|Default|GetIsMoving))
            (if (not (Variables|Default|GetIsOpen))
              (Variables|Default|SetHitbox1Enabled false)
              (bind _doorrotation (Timeline|DoorOpen2 PlayFromStart)
                (:Update
                  (Variables|Default|SetIsMoving true)
                  (Transformation|SetRelativeRotation (Variables|Default|GetDoor) (Class|KismetMathLibrary|NegateRotator (Math|Rotator|MakeRotator 0.0 0.0 (+ _doorrotation (.yaw (Variables|Default|GetInitial%20Rotation))))) false false))
                (:Finished
                  (Variables|Default|SetIsMoving false)
                  (Variables|Default|SetIsOpen true)))))))
      (else
        (Development|PrintString "gate lock 2 est false")))))

(event Input|ActionEvents|InputActionInteract
  (params (Key :type Key%20Structure))
  ;[1 1 1] Check if gate can be opened
  (:Pressed
    (if (Variables|Default|GetGateLock1)
      ;[1 1 1] If player interacts with the door and the door is not moving or closed
      (Utilities|FlowControl|Gate true
        (:Exit
          (if (not (Variables|Default|GetIsMoving))
            (if (not (Variables|Default|GetIsOpen))
              (Variables|Default|SetHitbox2Enabled false)
              (bind _doorrotation (Timeline|DoorOpen PlayFromStart)
                (:Update
                  (Variables|Default|SetIsMoving true)
                  (Transformation|SetRelativeRotation (Variables|Default|GetDoor) (Math|Rotator|MakeRotator 0.0 0.0 (+ _doorrotation (.yaw (Variables|Default|GetInitial%20Rotation)))) false false))
                (:Finished
                  (Variables|Default|SetIsMoving false)
                  (Variables|Default|SetIsOpen true)))))))
      (else
        (Development|PrintString "gate lock 1 est false")))))

(fn ConstructionScript
  (bind _returnvalue (Transformation|GetActorRotation))
  (Transformation|SetActorRotation _returnvalue)
  (Variables|Default|SetInitial%20Rotation _returnvalue))