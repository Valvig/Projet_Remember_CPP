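; ItemRemember is an interactible item actor that carries stat modifiers and makes itself known to a nearby RememberCharacter.
; On BeginPlay it packs sanity, walk speed, strength, range, attack speed cooldown and defense values into StatsModifierArray in a fixed index order.
; Its Sphere overlap events add the item to the character's ItemsClose list on entry and remove it on exit.
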(event OnComponentBeginOverlap(Sphere)
  (params (OverlappedComponent :type Primitive%20Component%20Object%20Reference) (OtherActor :type Actor%20Object%20Reference) (OtherComp :type Primitive%20Component%20Object%20Reference) (OtherBodyIndex :type Integer) (bFromSweep :type Boolean) (SweepResult :type Hit%20Result%20Structure%20%28by%20ref%29))
  (bind _asremember_character (Utilities|Casting|CastToRememberCharacter OtherActor))
  (Utilities|Array|AddUnique (Variables|/Game/blueprints/Character/RememberCharacter.RememberCharacter_C|GetItemsClose _asremember_character) self))

(event OnComponentEndOverlap(Sphere)
  (params (OverlappedComponent :type Primitive%20Component%20Object%20Reference) (OtherActor :type Actor%20Object%20Reference) (OtherComp :type Primitive%20Component%20Object%20Reference) (OtherBodyIndex :type Integer))
  (bind _asremember_character (Utilities|Casting|CastToRememberCharacter OtherActor))
  (Utilities|Array|RemoveItem (Variables|/Game/blueprints/Character/RememberCharacter.RememberCharacter_C|GetItemsClose _asremember_character) self))

(event EventBeginPlay
  (Utilities|Array|SetArrayElem (Variables|StatsModifier|GetStats%20Modifier%20Array) 0 (Variables|Statsmodifier|GetSanity))
  (Utilities|Array|SetArrayElem (Variables|StatsModifier|GetStats%20Modifier%20Array) 1 (Variables|Statsmodifier|GetWalk%20speed%20bonus))
  (Utilities|Array|SetArrayElem (Variables|StatsModifier|GetStats%20Modifier%20Array) 2 (Variables|Statsmodifier|GetStrength))
  (Utilities|Array|SetArrayElem (Variables|StatsModifier|GetStats%20Modifier%20Array) 3 (Variables|Statsmodifier|GetRange))
  (Utilities|Array|SetArrayElem (Variables|StatsModifier|GetStats%20Modifier%20Array) 4 (Variables|Statsmodifier|GetAttack%20speed%20%28cooldown%29))
  (Utilities|Array|SetArrayElem (Variables|StatsModifier|GetStats%20Modifier%20Array) 5 (Variables|Statsmodifier|GetDefense%20bonus)))

(event Collision|EventActorBeginOverlap
  (params (OtherActor :type Actor%20Object%20Reference)))

(event EventTick
  (params (DeltaSeconds :type Float%20%28single-precision%29)))

(fn ConstructionScript)