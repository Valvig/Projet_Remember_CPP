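; Base Blueprint for interactible weapons that carry stat modifiers and register with nearby player characters.
; On BeginPlay it copies its stat variables, such as sanity, strength, range and defense, into a name-keyed StatsModifierArray map.
; A Sphere overlap adds the weapon uniquely to a RememberCharacter's WeaponClose list and removes it when the overlap ends, printing debug strings for both.
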(event OnComponentBeginOverlap(Sphere)
  (params (OverlappedComponent :type Primitive%20Component%20Object%20Reference) (OtherActor :type Actor%20Object%20Reference) (OtherComp :type Primitive%20Component%20Object%20Reference) (OtherBodyIndex :type Integer) (bFromSweep :type Boolean) (SweepResult :type Hit%20Result%20Structure%20%28by%20ref%29))
  (bind _asremember_character (Utilities|Casting|CastToRememberCharacter OtherActor))
  (Utilities|Array|AddUnique (Variables|/Game/blueprints/Character/RememberCharacter.RememberCharacter_C|GetWeaponClose _asremember_character) self)
  (Development|PrintString "add"))

(event OnComponentEndOverlap(Sphere)
  (params (OverlappedComponent :type Primitive%20Component%20Object%20Reference) (OtherActor :type Actor%20Object%20Reference) (OtherComp :type Primitive%20Component%20Object%20Reference) (OtherBodyIndex :type Integer))
  (bind _asremember_character (Utilities|Casting|CastToRememberCharacter OtherActor))
  (Utilities|Array|RemoveItem (Variables|/Game/blueprints/Character/RememberCharacter.RememberCharacter_C|GetWeaponClose _asremember_character) self)
  (Development|PrintString "remove"))

(event EventBeginPlay
  (bind _statsmodifierarray (Variables|Default|GetStatsModifierArray))
  (Utilities|Map|Add _statsmodifierarray "Sanity" (Variables|Default|GetSanity))
  (Utilities|Map|Add _statsmodifierarray "WalkSpeed" (Variables|Default|GetWalkSpeedBonus))
  (Utilities|Map|Add _statsmodifierarray "Strength" (Variables|Default|GetStrength))
  (Utilities|Map|Add _statsmodifierarray "Range" (Variables|Default|GetRange))
  (Utilities|Map|Add _statsmodifierarray "AttackSpeed" (Variables|Default|GetAttackSpeed%28Cooldown%29))
  (Utilities|Map|Add _statsmodifierarray "Defense" (Variables|Default|GetDefenseBonus))
  (Utilities|Map|Add _statsmodifierarray "MaxSanity" (Variables|Default|GetMaxSanity)))

(fn ConstructionScript)