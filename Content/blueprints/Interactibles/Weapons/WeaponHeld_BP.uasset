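; WeaponHeld_BP is the held weapon Blueprint, which currently has no active behavior.
; Its BeginPlay and construction script are empty.
; Disconnected prototype logic checks whether the player's RememberCharacter is attacking and the weapon overlaps an EnemyFollower_BP mesh.
; That unreachable branch would deal damage equal to the player's Strength stat, with debug prints.
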(event EventBeginPlay)

(fn ConstructionScript)