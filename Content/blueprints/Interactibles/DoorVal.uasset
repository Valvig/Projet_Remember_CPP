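; Interactable two-sided door that RememberCharacter opens with the Interact input while inside either of its two hitboxes.
; Each side plays its own timeline to drive door yaw, with input enabled on entering a box while the door is shut.
; Overlap flags track passage between boxes, so leaving the final box swings the door closed according to its yaw sign, then resets flags and disables input.
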(event OnComponentBeginOverlap(DoorHitbox1)
  (params (OverlappedComponent :type Primitive%20Component%20Object%20Reference) (OtherActor :type Actor%20Object%20Reference) (OtherComp :type Primitive%20Component%20Object%20Reference) (OtherBodyIndex :type Integer) (bFromSweep :type Boolean) (SweepResult :type Hit%20Result%20Structure%20%28by%20ref%29))
  (Development|PrintString "In 1")
  (Utilities|Casting|CastToRememberCharacter OtherActor)
  (if (Variables|Default|GetIsOpen)
    (Variables|Default|SetIsInSecondBox true)
    (else
      (Input|EnableInput (Game|GetPlayerController 0))
      (Variables|Default|SetIsInFirstBox true)))
  (Variables|Default|SetIsInBox1 true))

(event OnComponentEndOverlap(DoorHitbox1)
  (params (OverlappedComponent :type Primitive%20Component%20Object%20Reference) (OtherActor :type Actor%20Object%20Reference) (OtherComp :type Primitive%20Component%20Object%20Reference) (OtherBodyIndex :type Integer))
  (Development|PrintString "JE SORS 1")
  (Utilities|Casting|CastToRememberCharacter OtherActor)
  (if (Variables|Default|GetIsMoving)
    (Utilities|FlowControl|Delay 0.4))
  (if (Variables|Default|GetIsInSecondBox)
    (Utilities|ResetBool)
    (else
      (Math|Float|CompareFloat (.yaw (Variables|/Script/Engine.SceneComponent|GetRelativeRotation (Variables|Default|GetDoor))) 0.0
        (:>
          (Variables|Default|SetIsMoving true)
          (bind _doorrotation (Timeline|CloseDoor90 PlayFromStart)
            (:Update
              (Utilities|SetRotationDoor _doorrotation))
            (:Finished
              (Variables|Default|SetIsMoving false :!label _label)
              (Utilities|ResetBool :!label _label_2)
              (Input|DisableInput (Game|GetPlayerController 0)))))
        (:==
          (goto _label_2))
        (:<
          (Variables|Default|SetIsMoving true)
          (bind _doorrotation_2 (Timeline|CloseDoor-90 PlayFromStart)
            (:Update
              (Utilities|SetRotationDoor _doorrotation_2))
            (:Finished
              (goto _label))))))))

(event OnComponentBeginOverlap(DoorHitbox2)
  (params (OverlappedComponent :type Primitive%20Component%20Object%20Reference) (OtherActor :type Actor%20Object%20Reference) (OtherComp :type Primitive%20Component%20Object%20Reference) (OtherBodyIndex :type Integer) (bFromSweep :type Boolean) (SweepResult :type Hit%20Result%20Structure%20%28by%20ref%29))
  (Development|PrintString "In 2")
  (Utilities|Casting|CastToRememberCharacter OtherActor)
  (if (Variables|Default|GetIsOpen)
    (Variables|Default|SetIsInSecondBox true)
    (else
      (Input|EnableInput (Game|GetPlayerController 0))
      (Variables|Default|SetIsInFirstBox true)))
  (Variables|Default|SetIsInBox2 true))

(event OnComponentEndOverlap(DoorHitbox2)
  (params (OverlappedComponent :type Primitive%20Component%20Object%20Reference) (OtherActor :type Actor%20Object%20Reference) (OtherComp :type Primitive%20Component%20Object%20Reference) (OtherBodyIndex :type Integer))
  (Development|PrintString "JE SORS 2")
  (Utilities|Casting|CastToRememberCharacter OtherActor)
  (if (Variables|Default|GetIsMoving)
    (Utilities|FlowControl|Delay 0.4))
  (if (Variables|Default|GetIsInSecondBox)
    (Utilities|ResetBool)
    (else
      (Math|Float|CompareFloat (.yaw (Variables|/Script/Engine.SceneComponent|GetRelativeRotation (Variables|Default|GetDoor))) 0.0
        (:>
          (Variables|Default|SetIsMoving true)
          (bind _doorrotation (Timeline|CloseDoor90 PlayFromStart)
            (:Update
              (Utilities|SetRotationDoor _doorrotation))
            (:Finished
              (Variables|Default|SetIsMoving false :!label _label)
              (Utilities|ResetBool :!label _label_2)
              (Input|DisableInput (Game|GetPlayerController 0)))))
        (:==
          (goto _label_2))
        (:<
          (Variables|Default|SetIsMoving true)
          (bind _doorrotation_2 (Timeline|CloseDoor-90 PlayFromStart)
            (:Update
              (Utilities|SetRotationDoor _doorrotation_2))
            (:Finished
              (goto _label))))))))

(event Input|ActionEvents|InputActionInteract
  (params (Key :type Key%20Structure))
  (:Pressed
    (if (not (Variables|Default|GetIsMoving))
      (if (== (.yaw (Variables|/Script/Engine.SceneComponent|GetRelativeRotation (Variables|Default|GetDoor))) 0.0)
        (if (Variables|Default|GetIsInBox1)
          (Variables|Default|SetIsMoving true)
          (bind _doorrotation (Timeline|DoorTImeline+ PlayFromStart)
            (:Update
              (Utilities|SetRotationDoor _doorrotation))
            (:Finished
              (Variables|Default|SetIsMoving false :!label _label)
              (Variables|Default|SetIsOpen true)))
          (elif (Variables|Default|GetIsInBox2)
            (Variables|Default|SetIsMoving true)
            (bind _doorrotation_2 (Timeline|DoorTimeline- PlayFromStart)
              (:Update
                (Utilities|SetRotationDoor _doorrotation_2))
              (:Finished
                (goto _label)))))))))

(fn ConstructionScript)