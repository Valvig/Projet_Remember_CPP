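; Parent Blueprint for items that carry stat modifiers and can be detected by a nearby RememberCharacter.
; On BeginPlay it packs its stat variables, such as sanity, speed, combat and defense values, into the name-keyed StatsModifierArray.
; Sphere overlap events add and remove the item from the character's ItemsClose list.
; Pickup and application of the modifiers are not handled here.
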(event OnComponentBeginOverlap(Sphere)
  (params (OverlappedComponent :type Primitive%20Component%20Object%20Reference) (OtherActor :type Actor%20Object%20Reference) (OtherComp :type Primitive%20Component%20Object%20Reference) (OtherBodyIndex :type Integer) (bFromSweep :type Boolean) (SweepResult :type Hit%20Result%20Structure%20%28by%20ref%29))
  (bind _asremember_character (Utilities|Casting|CastToRememberCharacter OtherActor))
  (Utilities|Array|AddUnique (Variables|/Game/blueprints/Character/RememberCharacter.RememberCharacter_C|GetItemsClose _asremember_character) self))

(event OnComponentEndOverlap(Sphere)
  (params (OverlappedComponent :type Primitive%20Component%20Object%20Reference) (OtherActor :type Actor%20Object%20Reference) (OtherComp :type Primitive%20Component%20Object%20Reference) (OtherBodyIndex :type Integer))
  (bind _asremember_character (Utilities|Casting|CastToRememberCharacter OtherActor))
  (Utilities|Array|RemoveItem (Variables|/Game/blueprints/Character/RememberCharacter.RememberCharacter_C|GetItemsClose _asremember_character) self))

(event EventBeginPlay
  (Utilities|Map|Add (Variables|StatsModifier|GetStats%20Modifier%20Array) "Sanity" (Variables|Statsmodifier|GetSanity))
  (Utilities|Map|Add (Variables|StatsModifier|GetStats%20Modifier%20Array) "WalkSpeed" (Variables|Statsmodifier|GetWalk%20speed%20bonus))
  (Utilities|Map|Add (Variables|StatsModifier|GetStats%20Modifier%20Array) "Strength" (Variables|Statsmodifier|GetStrength))
  (Utilities|Map|Add (Variables|StatsModifier|GetStats%20Modifier%20Array) "Range" (Variables|Statsmodifier|GetRange))
  (Utilities|Map|Add (Variables|StatsModifier|GetStats%20Modifier%20Array) "AttackSpeed" (Variables|Statsmodifier|GetAttack%20speed%20%28cooldown%29))
  (Utilities|Map|Add (Variables|StatsModifier|GetStats%20Modifier%20Array) "Defense" (Variables|Statsmodifier|GetDefense%20bonus))
  (Utilities|Map|Add (Variables|StatsModifier|GetStats%20Modifier%20Array) "MaxSanity" (Variables|StatsModifier|GetMaxSanity)))

(event EventTick
  (params (DeltaSeconds :type Float%20%28single-precision%29)))

(fn ConstructionScript)