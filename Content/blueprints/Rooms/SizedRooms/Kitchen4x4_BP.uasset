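; Kitchen4x4_BP is a tile-sized kitchen room that orients itself on BeginPlay and hands enemy spawn points to its fog cube.
; It rotates Arrow1 by Orientation, then shifts the root by room size and tile size for yaw 0, 180 or 270.
; Only in those cases, it records skeletal mesh placeholder transforms, destroys the meshes, then passes the list to the FogCube child actor and calls SpawnInitial.
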(event Collision|EventActorBeginOverlap
  (params (OtherActor :type Actor%20Object%20Reference))
  (|CallParentFunction OtherActor) ; This node is disabled and will not be called.\nDrag off pins to build functionality.
)

(event EventTick
  (params (DeltaSeconds :type Float%20%28single-precision%29))
  (|CallParentFunction DeltaSeconds) ; This node is disabled and will not be called.\nDrag off pins to build functionality.
)

(event EventBeginPlay
  (bind _orientation (Variables|Default|GetOrientation))
  (bind _skeletalstodestroy (Variables|Default|GetSkeletalsToDestroy))
  (bind _ennemyplaceholders (Variables|Default|GetEnnemyPlaceholders))
  (bind _defaultsceneroot (Variables|Default|GetDefaultSceneRoot))
  (|CallParentFunction)
  (Transformation|AddWorldRotation (Variables|Default|GetArrow1) (Variables|Default|GetOrientation) false false)
  (if (== (.yaw _orientation) 0.0)
    (Transformation|AddRelativeLocation _defaultsceneroot (Math|Vector|MakeVector 0.0 (* (* (- (Variables|Default|GetYSize) 1) -1.0) (Variables|Default|GetTileSize)) 0.0) false false)
    ;[0 0.1932 0.6281] Ennemy Positions Settings
    (for _array_element (Components|GetChildrenComponents (Variables|Transformation|GetRootComponent) true) :!label _label
      (bind _asskeletal_mesh_component (Utilities|Casting|CastToSkeletalMeshComponent _array_element))
      (Utilities|Array|Add (Variables|Default|GetSkeletalsToDestroy) _asskeletal_mesh_component)
      (Utilities|Array|Add _ennemyplaceholders (Utilities|Struct|MakeEnnemyPlaceholders (Transformation|GetWorldLocation _asskeletal_mesh_component) (Transformation|GetWorldRotation _asskeletal_mesh_component) (Transformation|GetWorldScale _asskeletal_mesh_component))))
    (for _index (range 0 (- (Utilities|Array|Length _skeletalstodestroy) 1))
      (Components|DestroyComponent (Utilities|Array|Get(acopy) _skeletalstodestroy _index)))
    (bind _asfog_cube (Utilities|Casting|CastToFogCube (Variables|/Script/Engine.ChildActorComponent|GetChildActor (Variables|Default|GetFogCube))))
    (Variables|/Game/blueprints/Fog/FogCube.FogCube_C|SetPositions _asfog_cube _ennemyplaceholders)
    (Default|SpawnInitial _asfog_cube)
    (elif (== (.yaw _orientation) 1.8e+02)
      (Transformation|AddRelativeLocation _defaultsceneroot (Math|Vector|MakeVector (* (* (- (Variables|Default|GetXsize) 1) -1.0) (Variables|Default|GetTileSize)) 0.0 0.0) false false)
      (goto _label)
      (elif (== (.yaw _orientation) 2.7e+02)
        (Transformation|AddRelativeLocation (Variables|Default|GetDefaultSceneRoot) (Math|Vector|MakeVector (* (* (- (Variables|Default|GetXsize) 1) -1.0) (Variables|Default|GetTileSize)) (* (* (- (Variables|Default|GetYSize) 1) -1.0) (Variables|Default|GetTileSize)) 0.0) false false)
        (goto _label)))))

(fn ConstructionScript
  (|CallParentFunction))