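; StartRoom4x4_BP is a room Blueprint, named as a 4x4 start room, that builds on a parent room class.
; BeginPlay runs the parent logic, then rotates the Arrow component by Orientation, and the construction script only calls its parent.
; An unconnected chain would offset the root by room size times TileSize for yaws of 90, 180 and 270, but it never runs.
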(event EventBeginPlay
  (|CallParentFunction)
  (Transformation|AddWorldRotation (Variables|Default|GetArrow) (Variables|Default|GetOrientation) false false))

(fn ConstructionScript
  (|CallParentFunction))