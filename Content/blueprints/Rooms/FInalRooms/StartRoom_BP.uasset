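; Start room Blueprint for a tile-based layout that rotates its contents to a given orientation when play begins.
; After the parent's BeginPlay, it adds a visible arrow component at the center of the tile at first column, last row, computed from TileSize and YSize.
; It attaches all static meshes and DoorNoInteraction to that arrow, keeping world transforms, then rotates the arrow by Orientation so it acts as a runtime pivot.
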(event EventBeginPlay
  (|CallParentFunction)
  (bind _returnvalue (AddComponent|AddArrowComponent false (Math|Transform|MakeTransform (Math|Vector|MakeVector (/ (Variables|Default|GetTileSize) 2.0) (+ (/ (Variables|Default|GetTileSize) 2.0) (* (- (Variables|Default|GetYSize) 1) (Variables|Default|GetTileSize))) 0.0) "0, 0, 0" "1,1,1")))
  (bind _asarrow_component (Utilities|Casting|CastToArrowComponent _returnvalue))
  (Development|SetHiddeninGame _asarrow_component false false)
  (for _array_element (Actor|GetComponentsByClass "/Script/Engine.StaticMeshComponent")
    (Transformation|AttachComponentToComponent _array_element _returnvalue "None" "KeepWorld" "KeepWorld" "KeepWorld" true))
  (Transformation|AttachComponentToComponent (Variables|Default|GetDoorNoInteraction) _returnvalue "None" "KeepWorld" "KeepWorld" "KeepWorld" true)
  (Transformation|AddWorldRotation _returnvalue (Variables|Default|GetOrientation) false false))

(fn ConstructionScript
  (|CallParentFunction))