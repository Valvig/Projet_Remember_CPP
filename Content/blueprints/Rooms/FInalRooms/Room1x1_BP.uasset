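; A 1x1 room Blueprint that orients itself and seeds enemy spawns on BeginPlay.
; It adds an arrow component as a tile-based pivot, attaches the static meshes, fog cube and door to it, then rotates it by Orientation.
; Skeletal meshes under the root act as editor-placed enemy placeholders: their world transforms are recorded, then the meshes are destroyed.
; The FogCube child actor receives those transforms and runs its initial spawn.
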(event EventBeginPlay
  (bind _skeletalstodestroy (Variables|Default|GetSkeletalsToDestroy))
  (bind _ennemyplaceholders (Variables|Default|GetEnnemyPlaceholders))
  (|CallParentFunction)
  (bind _returnvalue (AddComponent|AddArrowComponent false (Math|Transform|MakeTransform (Math|Vector|MakeVector (/ (Variables|Default|GetTileSize) 2.0) (+ (/ (Variables|Default|GetTileSize) 2.0) (* (- (Variables|Default|GetYSize) 1) (Variables|Default|GetTileSize))) 0.0) "0, 0, 0" "1,1,1")))
  (bind _asarrow_component (Utilities|Casting|CastToArrowComponent _returnvalue))
  (Development|SetHiddeninGame _asarrow_component false false)
  (for _array_element (Actor|GetComponentsByClass "/Script/Engine.StaticMeshComponent")
    (Transformation|AttachComponentToComponent _array_element _returnvalue "None" "KeepWorld" "KeepWorld" "KeepWorld" true))
  (Transformation|AttachComponentToComponent (Variables|Default|GetFogCube) _returnvalue "None" "KeepWorld" "KeepWorld" "KeepWorld" true)
  (Transformation|AttachComponentToComponent (Variables|Default|GetDoorNoInteraction) _returnvalue "None" "KeepWorld" "KeepWorld" "KeepWorld" true)
  (Transformation|AddWorldRotation _returnvalue (Variables|Default|GetOrientation) false false)
  ;[0 0.1932 0.6281] Ennemy Positions Settings
  (for _array_element_2 (Components|GetChildrenComponents (Variables|Transformation|GetRootComponent) false)
    (bind _asskeletal_mesh_component (Utilities|Casting|CastToSkeletalMeshComponent _array_element_2))
    (Utilities|Array|Add (Variables|Default|GetSkeletalsToDestroy) _asskeletal_mesh_component)
    (Utilities|Array|Add _ennemyplaceholders (Utilities|Struct|MakeEnnemyPlaceholders (Transformation|GetWorldLocation _asskeletal_mesh_component) (Transformation|GetWorldRotation _asskeletal_mesh_component) (Transformation|GetWorldScale _asskeletal_mesh_component))))
  (for _index (range 0 (- (Utilities|Array|Length _skeletalstodestroy) 1))
    (Components|DestroyComponent (Utilities|Array|Get(acopy) _skeletalstodestroy _index)))
  (bind _asfog_cube (Utilities|Casting|CastToFogCube (Variables|/Script/Engine.ChildActorComponent|GetChildActor (Variables|Default|GetFogCube))))
  (Variables|/Game/blueprints/Fog/FogCube.FogCube_C|SetPositions _asfog_cube _ennemyplaceholders)
  (Default|SpawnInitial _asfog_cube))

(fn ConstructionScript
  (|CallParentFunction))