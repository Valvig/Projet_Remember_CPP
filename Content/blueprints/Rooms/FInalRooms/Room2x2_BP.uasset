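; Grid-based room actor, apparently a 2x2 piece, that orients itself when play begins.
; BeginPlay rotates the root by Orientation, then for 180, 90 or 270 degree yaw applies a relative offset derived from Xsize, YSize and TileSize to compensate for the turn.
; The 180 case also prints a debug string.
; An unwired alternative that re-parents meshes under a runtime arrow pivot remains in the graph.
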(event EventBeginPlay
  (bind _orientation (Variables|Default|GetOrientation))
  (bind _tilesize (Variables|Default|GetTileSize))
  (|CallParentFunction)
  (Transformation|AddWorldRotation (Variables|Default|GetDefaultSceneRoot) (Variables|Default|GetOrientation) false false)
  (if (== (.yaw _orientation) 1.8e+02)
    (Transformation|AddRelativeLocation (Variables|Default|GetDefaultSceneRoot) (Math|Vector|MakeVector (* (- (Variables|Default|GetXsize) 1) _tilesize) (* (Variables|Default|GetYSize) _tilesize) 0.0) false false)
    (Development|PrintString "Bas")
    (elif (== (.yaw _orientation) 9e+01)
      (Transformation|AddRelativeLocation (Variables|Default|GetDefaultSceneRoot) (Math|Vector|MakeVector (* (Variables|Default|GetYSize) (Variables|Default|GetTileSize)) 0.0 0.0) false false)
      (elif (== (.yaw _orientation) 2.7e+02)
        (Transformation|AddRelativeLocation (Variables|Default|GetDefaultSceneRoot) (Math|Vector|MakeVector 0.0 (* (- (Variables|Default|GetXsize) 1) (Variables|Default|GetTileSize)) 0.0) false false)))))

(event Collision|EventActorBeginOverlap
  (params (OtherActor :type Actor%20Object%20Reference))
  (|CallParentFunction OtherActor) ; This node is disabled and will not be called.\nDrag off pins to build functionality.
)

(event EventTick
  (params (DeltaSeconds :type Float%20%28single-precision%29))
  (|CallParentFunction DeltaSeconds) ; This node is disabled and will not be called.\nDrag off pins to build functionality.
)

(fn ConstructionScript
  (|CallParentFunction))