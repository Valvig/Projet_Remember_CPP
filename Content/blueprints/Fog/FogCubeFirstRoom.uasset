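; Fog volume for the first room that thins out while the RememberCharacter is inside it and returns when they leave.
; The construction script makes a dynamic instance of the FogFirstRoom material on the static mesh.
; Overlap events toggle HideFog, and Tick ramps the material's Density parameter down or up within limits, scaled by frame time.
; An unused branch that sank and raised the mesh instead remains disconnected.
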(event Collision|EventActorBeginOverlap
  (params (OtherActor :type Actor%20Object%20Reference))
  (Utilities|Casting|CastToRememberCharacter OtherActor)
  (Variables|Default|SetHideFog true))

(event Collision|EventActorEndOverlap
  (params (OtherActor :type Actor%20Object%20Reference))
  (Utilities|Casting|CastToRememberCharacter OtherActor)
  (Variables|Default|SetHideFog false))

(event EventTick
  (params (DeltaSeconds :type Float%20%28single-precision%29))
  (bind _dynamicmaterial (Variables|Default|GetDynamicMaterial))
  (bind _dynamicmaterial_2 (Variables|Default|GetDynamicMaterial))
  (Variables|Default|SetDeltaTime DeltaSeconds)
  (if (Variables|Default|GetHideFog)
    (bind _returnvalue (Rendering|Material|GetScalarParameterValue _dynamicmaterial "Density" :!class /Script/Engine.MaterialInstanceDynamic))
    (if (>= _returnvalue 0.0)
      (Rendering|Material|SetScalarParameterValue _dynamicmaterial "Density" (- _returnvalue (* (* (Variables|Default|GetDeltaTime) 1e+02) (Variables|Default|GetScaleParameterValue))) :!class /Script/Engine.MaterialInstanceDynamic))
    (else
      (bind _returnvalue_2 (Rendering|Material|GetScalarParameterValue _dynamicmaterial_2 "Density" :!class /Script/Engine.MaterialInstanceDynamic))
      (if (<= _returnvalue_2 4.0)
        (Rendering|Material|SetScalarParameterValue _dynamicmaterial_2 "Density" (+ _returnvalue_2 (* (* (Variables|Default|GetDeltaTime) 1e+02) (Variables|Default|GetScaleParameterValue))) :!class /Script/Engine.MaterialInstanceDynamic)))))

(fn ConstructionScript
  (bind _returnvalue (Rendering|Material|CreateDynamicMaterialInstance (Variables|Default|GetStaticMesh) 0 "/Game/blueprints/Fog/FogFirstRoom.FogFirstRoom" "None" :!class /Script/Engine.PrimitiveComponent))
  (Variables|Default|SetDynamicMaterial _returnvalue))