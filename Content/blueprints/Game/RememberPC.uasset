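; RememberPC is a player controller for click-to-move navigation with the cursor.
; SetDestination opens a gate while held, so each Tick traces under the cursor on the Visibility channel and passes the hit to MoveToHitLocation, which calls SimpleMoveToLocation.
; A Z comparison skips hits at exactly zero height, which also covers empty traces.
; Debug prints of the hit's X and Y are left unconnected.
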(event EventTick
  (params (DeltaSeconds :type Float%20%28single-precision%29))
  (bind _hitresult (Game|Player|GetHitResultUnderCursorbyChannel "TraceTypeQuery1" true))
  (Utilities|FlowControl|Gate true
    (:Exit
      (Math|Float|CompareFloat (.Z (Math|Vector|BreakVector (.Location (Collision|BreakHitResult _hitresult)))) 0.0
        (:>
          _)
        (:<
          _))
      (CallFunction|MovetoHitLocation _hitresult))))

(event Input|ActionEvents|InputActionSetDestination
  (params (Key :type Key%20Structure))
  (bind _hitresult (Game|Player|GetHitResultUnderCursorbyChannel "TraceTypeQuery1" true))
  (:Pressed
    (Utilities|FlowControl|Gate true) ; enters at Open
  )
  (:Released
    (Utilities|FlowControl|Gate true) ; enters at Close
  ))

(fn ConstructionScript)

(fn MovetoHitLocation
  (params (Hit :type Hit%20Result%20Structure))
  (AI|Navigation|SimpleMovetoLocation self (.Location (Collision|BreakHitResult Hit))))