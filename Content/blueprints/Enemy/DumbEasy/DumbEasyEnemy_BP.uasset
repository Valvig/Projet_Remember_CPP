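; Blueprint for a basic "DumbEasy" enemy that attacks the RememberCharacter, takes damage and is destroyed when its health runs out.
; Attack, React and Hit events set animation flags, with attack state and the end of reactions written to the AI blackboard.
; Attacks apply damage through a multi-sphere trace around itself, and ending a reaction triggers an attack.
; Tick tracks speed; damage computes a knockback direction but applies no movement here.
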(event Custom|Attack
  ;[0.6377 0 0.1858] Attack Event Animation
  (Variables|Default|SetIsAttacking true)
  (AI|Components|Blackboard|SetValueasBool (AI|GetBlackboard (AI|GetAIController self)) (Variables|Default|GetKeyNameIsAttacking) true)
  (CallFunction|AttackDumbEasy))

(event Custom|EndAttack
  ;[0.6377 0 0.1858] Attack Event Animation
  (bind _output_get (Variables|Default|SetIsAttacking false))
  (AI|Components|Blackboard|SetValueasBool (AI|GetBlackboard (AI|GetAIController self)) (Variables|Default|GetKeyNameIsAttacking) _output_get))

(event Custom|React
  ;[0.0773 0.744 0] React Event Animation
  (Variables|Default|SetIsReacting true))

(event Custom|EndReact
  ;[0.0773 0.744 0] React Event Animation
  (bind _output_get (Variables|Default|SetIsReacting false))
  (AI|Components|Blackboard|SetValueasBool (AI|GetBlackboard (AI|GetAIController self)) (Variables|Default|GetKeyNameIsReacting) _output_get)
  (CallFunction|Attack))

(event Custom|AttackDumbEasy
  (params (Other%20Actor :type Actor%20Object%20Reference))
  (bind _returnvalue (Transformation|GetActorLocation))
  ;[0.4638 0 0.3618] Attack System
  (bind _outhits (Collision|MultiSphereTraceByChannel _returnvalue _returnvalue (Variables|Default|GetRange) "TraceTypeQuery3" false 0 "None" true "(R=1.000000,G=0.000000,B=0.000000,A=1.000000)" "(R=0.000000,G=1.000000,B=0.000000,A=1.000000)" 5e+02))
  (for _array_element _outhits
    (bind _asremember_character (Utilities|Casting|CastToRememberCharacter (.HitActor (Collision|BreakHitResult _array_element))))
    (Default|TakeDamageEvent _asremember_character self (Variables|Default|GetStrenght))))

(event Custom|TakeDamageEvent
  (params (Source%20of%20damage :type Actor%20Object%20Reference) (Damage%20taken%20value :type Float%20%28single-precision%29))
  ;[0 0.1546 0.6667] KnockBack and Damage Gestion
  (Variables|Default|SetCharacterLocation (Transformation|GetActorLocation Source%20of%20damage))
  (Variables|Default|SetTempLocation (Transformation|GetActorLocation))
  (Variables|Default|SetUnitDirectionVector (Math|Vector|GetUnitDirection(Vector) (Variables|Default|GetCharacterLocation) (Variables|Default|GetTempLocation)))
  (Variables|Default|SetHealthPoints (- (Variables|Default|GetHealthPoints) Damage%20taken%20value))
  (CallFunction|Hit)
  (if (<= (Variables|Default|GetHealthPoints) 0.0)
    (Actor|DestroyActor)))

(event Custom|Hit
  ;[0 0.02899 0.7923] Hit Event Animation
  (Variables|Default|SetIsHit true))

(event Custom|EndHit
  ;[0 0.02899 0.7923] Hit Event Animation
  (Variables|Default|SetIsHit false))

(event EventTick
  (params (DeltaSeconds :type Float%20%28single-precision%29))
  ;[0.3672 0 0.4595] Set Speed
  (Variables|Default|SetSpeed (Math|Vector|VectorLength (Transformation|GetVelocity))))

(fn ConstructionScript)