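; Static enemy Blueprint that attacks a RememberCharacter entering its AttackArea and can itself be killed.
; On overlap, if CanAttack is set, it waits a second, then runs a debug-drawn multi-sphere trace around itself, playing an attack animation and applying Strenght damage to RememberCharacter hits.
; The attack triggers only on overlap begin, with no repeat loop.
; TakeDamageEvent subtracts from HealthPoints and destroys the actor at zero or below.
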(event OnComponentBeginOverlap(AttackArea)
  (params (OverlappedComponent :type Primitive%20Component%20Object%20Reference) (OtherActor :type Actor%20Object%20Reference) (OtherComp :type Primitive%20Component%20Object%20Reference) (OtherBodyIndex :type Integer) (bFromSweep :type Boolean) (SweepResult :type Hit%20Result%20Structure%20%28by%20ref%29))
  (bind _returnvalue (Transformation|GetActorLocation))
  ;[0.4638 0 0.3618] Attack System
  (if (Variables|Default|GetCanAttack)
    (Utilities|Casting|CastToRememberCharacter OtherActor)
    (Utilities|FlowControl|Delay 1.0)
    (bind _outhits (Collision|MultiSphereTraceForObjects _returnvalue _returnvalue (Variables|Default|GetRange) (Utilities|Array|MakeArray "ObjectTypeQuery3") false 0 "ForDuration" true "(R=1.000000,G=0.000000,B=0.000000,A=1.000000)" "(R=0.000000,G=1.000000,B=0.000000,A=1.000000)" 1.0))
    (for _array_element _outhits
      (bind _asremember_character (Utilities|Casting|CastToRememberCharacter (.HitActor (Collision|BreakHitResult _array_element))))
      (Components|Animation|PlayAnimation (Variables|Character|GetMesh) "/Game/CharaRemember/Anims/attack2.attack2" false)
      (Default|TakeDamageEvent _asremember_character self (Variables|Default|GetStrenght)))
    (Development|PrintString "EnemyAttack")))

(event Custom|TakeDamageEvent
  (params (Source%20of%20damage :type Actor%20Object%20Reference) (Damage%20taken%20value :type Float%20%28single-precision%29))
  ;[0.4348 0.3865 0] Damage
  (Variables|Default|SetHealthPoints (- (Variables|Default|GetHealthPoints) Damage%20taken%20value))
  (if (<= (Variables|Default|GetHealthPoints) 0.0)
    (Actor|DestroyActor)))

(fn ConstructionScript)