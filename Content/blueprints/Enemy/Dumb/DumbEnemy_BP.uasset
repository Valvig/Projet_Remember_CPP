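; Dumb enemy that damages RememberCharacter on weapon overlap, reduced if it is blocking, and swaps its mesh material while that character is inside AttackArea.
; TakeDamageEvent subtracts health and plays a timeline that pushes the capsule horizontally away from the damage source with sweep, destroying the actor at zero health.
; Tick only draws a long-lived debug line tracing its path.
; Sine-based strafing movement using a blackboard end location is present but unwired.
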(event OnComponentBeginOverlap(Weapon)
  (params (OverlappedComponent :type Primitive%20Component%20Object%20Reference) (OtherActor :type Actor%20Object%20Reference) (OtherComp :type Primitive%20Component%20Object%20Reference) (OtherBodyIndex :type Integer) (bFromSweep :type Boolean) (SweepResult :type Hit%20Result%20Structure%20%28by%20ref%29))
  (bind _returnvalue (Components|GetOwner OverlappedComponent))
  (bind _asremember_character (Utilities|Casting|CastToRememberCharacter OtherActor))
  (if (Variables|/Game/blueprints/Character/RememberCharacter.RememberCharacter_C|GetIsBlocking _asremember_character)
    (Default|TakeDamageEvent _asremember_character _returnvalue (* (Variables|Default|GetStrenght) 0.2))
    (else
      (Default|TakeDamageEvent _asremember_character _returnvalue (Variables|Default|GetStrenght)))))

(event OnComponentBeginOverlap(AttackArea)
  (params (OverlappedComponent :type Primitive%20Component%20Object%20Reference) (OtherActor :type Actor%20Object%20Reference) (OtherComp :type Primitive%20Component%20Object%20Reference) (OtherBodyIndex :type Integer) (bFromSweep :type Boolean) (SweepResult :type Hit%20Result%20Structure%20%28by%20ref%29))
  (Utilities|Casting|CastToRememberCharacter OtherActor)
  (Rendering|Material|SetMaterial (Variables|Character|GetMesh) 0 "/Game/StarterContent/Materials/M_Metal_Burnished_Steel.M_Metal_Burnished_Steel"))

(event OnComponentEndOverlap(AttackArea)
  (params (OverlappedComponent :type Primitive%20Component%20Object%20Reference) (OtherActor :type Actor%20Object%20Reference) (OtherComp :type Primitive%20Component%20Object%20Reference) (OtherBodyIndex :type Integer))
  (Utilities|Casting|CastToRememberCharacter OtherActor)
  (Rendering|Material|SetMaterial (Variables|Character|GetMesh) 0 "/Game/CharaRemember/Materials/Chara.Chara"))

(event Custom|TakeDamageEvent
  (params (Source%20of%20damage :type Actor%20Object%20Reference) (Damage%20taken%20value :type Float%20%28single-precision%29))
  ;[0 0.1546 0.6667] KnockBack and Damage Gestion
  (Variables|Default|SetCharacterLocation (Transformation|GetActorLocation Source%20of%20damage))
  (Variables|Default|SetTempLocation (Transformation|GetActorLocation))
  (Variables|Default|SetUnitDirectionVector (Math|Vector|GetUnitDirection(Vector) (Variables|Default|GetCharacterLocation) (Variables|Default|GetTempLocation)))
  (Variables|Default|SetHealthPoints (- (Variables|Default|GetHealthPoints) Damage%20taken%20value))
  (bind _newtrack_0 (Timeline|Timeline_1 PlayFromStart)
    (:Update
      (bind _output_get (Variables|Default|SetTempLocation (Math|Vector|MakeVector (.x (+ (Variables|Default|GetTempLocation) (* (Variables|Default|GetUnitDirectionVector) (* _newtrack_0 25.0)))) (.y (+ (Variables|Default|GetTempLocation) (* (Variables|Default|GetUnitDirectionVector) (* _newtrack_0 25.0)))) (.z (Variables|Default|GetTempLocation)))))
      (Transformation|SetWorldLocation (Variables|Collision|GetCapsuleComponent) _output_get true false)
      (if (<= (Variables|Default|GetHealthPoints) 0.0)
        (Actor|DestroyActor)))))

(event EventTick
  (params (DeltaSeconds :type Float%20%28single-precision%29))
  (bind _returnvalue (Transformation|GetActorLocation))
  ;[0.3672 0 0.4595] Draw Debug Lin to check the curve
  (Rendering|Debug|DrawDebugLine _returnvalue (+ _returnvalue 1e+01) "(R=1.000000,G=0.000000,B=0.552450,A=1.000000)" 5e+02 0.0))

(fn ConstructionScript)