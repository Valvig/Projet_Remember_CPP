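; Behavior tree service that picks a random point around the enemy as a blackboard location, apparently for wandering.
; On activation it flattens a random unit vector to XY without renormalizing, scales it by a random LengthArray entry and adds the owner's location.
; It writes the result to the Location key.
; A debug print rolls the length separately, so its value can differ from the stored one.
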(event EventReceiveActivationAI
  (params (OwnerController :type AI%20Controller%20Object%20Reference) (ControlledPawn :type Pawn%20Object%20Reference))
  (bind _returnvalue (Math|Random|RandomUnitVector))
  (bind _lengtharray (Variables|Default|GetLengthArray))
  (bind _output_get (Variables|Default|SetDirectionValue (Math|Vector|MakeVector (.x _returnvalue) (.y _returnvalue) 0.0)))
  (Development|PrintString (Utilities|String|ToString(Vector) (+ (* _output_get (Utilities|Array|Get(acopy) _lengtharray (Math|Random|RandomIntegerinRange 0 (- (Utilities|Array|Length _lengtharray) 1)))) (Transformation|GetActorLocation (Components|GetOwner (Class|BTFunctionLibrary|GetOwnerComponent))))))
  (Variables|Default|SetLocationValue (+ (* _output_get (Utilities|Array|Get(acopy) _lengtharray (Math|Random|RandomIntegerinRange 0 (- (Utilities|Array|Length _lengtharray) 1)))) (Transformation|GetActorLocation (Components|GetOwner (Class|BTFunctionLibrary|GetOwnerComponent)))))
  (AI|BehaviorTree|SetBlackboardValueasVector (Variables|Default|GetLocation) (Variables|Default|GetLocationValue)))