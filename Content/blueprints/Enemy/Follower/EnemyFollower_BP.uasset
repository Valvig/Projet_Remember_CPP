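; Follower enemy Blueprint handling melee attacks on RememberCharacter and its own damage reactions.
; When attacks are allowed, entering AttackArea triggers a delayed forward box trace that plays the attack animation and deals Strenght-based damage.
; Weapon overlaps also deal damage, reduced if the character is blocking.
; TakeDamageEvent lowers health and runs a Timeline-driven, swept horizontal knockback away from the source, destroying the enemy at zero health.
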(event OnComponentBeginOverlap(Weapon)
  (params (OverlappedComponent :type Primitive%20Component%20Object%20Reference) (OtherActor :type Actor%20Object%20Reference) (OtherComp :type Primitive%20Component%20Object%20Reference) (OtherBodyIndex :type Integer) (bFromSweep :type Boolean) (SweepResult :type Hit%20Result%20Structure%20%28by%20ref%29))
  (bind _returnvalue (Components|GetOwner OverlappedComponent))
  (bind _asremember_character (Utilities|Casting|CastToRememberCharacter OtherActor))
  (if (Variables|/Game/blueprints/Character/RememberCharacter.RememberCharacter_C|GetIsBlocking _asremember_character)
    (Default|TakeDamageEvent _asremember_character _returnvalue (* (Variables|Default|GetStrenght) 0.2))
    (else
      (Default|TakeDamageEvent _asremember_character _returnvalue (Variables|Default|GetStrenght)))))

(event OnComponentBeginOverlap(AttackArea)
  (params (OverlappedComponent :type Primitive%20Component%20Object%20Reference) (OtherActor :type Actor%20Object%20Reference) (OtherComp :type Primitive%20Component%20Object%20Reference) (OtherBodyIndex :type Integer) (bFromSweep :type Boolean) (SweepResult :type Hit%20Result%20Structure%20%28by%20ref%29))
  (bind _returnvalue (Transformation|GetActorLocation))
  (bind _capsulecomponent (Variables|Default|GetCapsuleComponent))
  (bind _outradius (Components|Capsule|GetScaledCapsuleSize _capsulecomponent))
  ;[0.4638 0 0.3618] Attack System
  (if (Variables|Default|GetCanAttack)
    (Utilities|Casting|CastToRememberCharacter OtherActor)
    (Utilities|FlowControl|Delay 1.0)
    (bind _outhits (Class|KismetSystemLibrary|BoxTraceMulti _returnvalue (+ _returnvalue (* (Transformation|GetActorForwardVector) (Variables|Default|GetRange))) (Math|Vector|MakeVector _outradius _outradius _outradius) "0, 0, 0" "TraceTypeQuery3" false 0 "None" true))
    (for _array_element _outhits
      (bind _asremember_character (Utilities|Casting|CastToRememberCharacter (.HitActor (Collision|BreakHitResult _array_element))))
      (Components|Animation|PlayAnimation (Variables|Character|GetMesh) "/Game/CharaRemember/Anims/attack2.attack2" false)
      (Default|TakeDamageEvent _asremember_character self (Variables|Default|GetStrenght)))))

(event Custom|TakeDamageEvent
  (params (Source%20of%20damage :type Actor%20Object%20Reference) (Damage%20taken%20value :type Float%20%28single-precision%29))
  ;[0 0.1546 0.6667] KnockBack and Damage Gestion
  (Variables|Default|SetCharacterLocation (Transformation|GetActorLocation Source%20of%20damage))
  (Variables|Default|SetTempLocation (Transformation|GetActorLocation))
  (Variables|Default|SetUnitDirectionVector (Math|Vector|GetUnitDirection(Vector) (Variables|Default|GetCharacterLocation) (Variables|Default|GetTempLocation)))
  (Variables|Default|SetHealthPoints (- (Variables|Default|GetHealthPoints) Damage%20taken%20value))
  (bind _newtrack_0 (Timeline|Timeline_1 PlayFromStart)
    (:Update
      (bind _output_get (Variables|Default|SetTempLocation (Math|Vector|MakeVector (.x (+ (Variables|Default|GetTempLocation) (* (Variables|Default|GetUnitDirectionVector) (* _newtrack_0 25.0)))) (.y (+ (Variables|Default|GetTempLocation) (* (Variables|Default|GetUnitDirectionVector) (* _newtrack_0 25.0)))) (.z (Variables|Default|GetTempLocation)))))
      (Transformation|SetWorldLocation (Variables|Default|GetCapsuleComponent) _output_get true false)
      (if (<= (Variables|Default|GetHealthPoints) 0.0)
        (Actor|DestroyActor)))))

(fn ConstructionScript)